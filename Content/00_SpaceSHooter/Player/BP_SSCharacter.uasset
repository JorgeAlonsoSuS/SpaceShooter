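; Player character for a space shooter that moves, fires and loses lives when hit.
; Enhanced Input drives movement along the actor's right and forward axes, while firing spawns Ammo at ShootPoint behind a timer-based cooldown.
; Overlapping "Enemy"-tagged actors costs a life, notifying SS_GameMode when none remain.
; Overlapping "Shoot"-tagged actors shortens the fire cooldown down to a minimum limit.
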(event Custom|CanFire
  (Variables|Default|SetCanShoot true))

(event Custom|GetDamage
  (bind _output_get (Variables|Default|SetLifes (- (Variables|Default|GetLifes) 1)))
  (if (== _output_get 0)
    (bind _asss_game_mode (Utilities|Casting|CastToSS_GameMode (Game|GetGameMode)))
    (Default|PlayerDead _asss_game_mode)))

(event Input|EnhancedActionEvents|EnhancedInputActionBP_InputMove
  (params (ActionValue :type Vector%202D%20Structure) (ElapsedSeconds :type Float%20%28double-precision%29) (TriggeredSeconds :type Float%20%28double-precision%29) (InputAction :type Input%20Action%20Object%20Reference :default "/Game/00_SpaceSHooter/Inputs/BP_InputMove.BP_InputMove"))
  (Pawn|Input|AddMovementInput (Transformation|GetActorRightVector) (.x ActionValue) false)
  (Pawn|Input|AddMovementInput (Transformation|GetActorForwardVector) (.y ActionValue) false))

(event Input|EnhancedActionEvents|EnhancedInputActionBP_InputFire
  (params (ActionValue :type Boolean) (ElapsedSeconds :type Float%20%28double-precision%29) (TriggeredSeconds :type Float%20%28double-precision%29) (InputAction :type Input%20Action%20Object%20Reference :default "/Game/00_SpaceSHooter/Inputs/BP_InputFire.BP_InputFire"))
  (if (Variables|Default|GetCanShoot)
    (CallFunction|DoFire)
    (Variables|Default|SetCanShoot false)
    (Utilities|Time|SetTimerbyEvent (delegate Custom|CanFire) (Variables|Default|GetFireTemp))))

(event EventBeginPlay
  (bind _asplayer_controller (Utilities|Casting|CastToPlayerController (Pawn|GetController)))
  (Utilities|IsValid (PlayerController|LocalPlayerSubsystems|GetEnhancedInputLocalPlayerSubsystem _asplayer_controller)
    (:Is%20Valid
      (Input|AddMappingContext (PlayerController|LocalPlayerSubsystems|GetEnhancedInputLocalPlayerSubsystem _asplayer_controller) "/Game/00_SpaceSHooter/Inputs/BP_InputMapping.BP_InputMapping" 0 "(bIgnoreAllPressedKeysUntilRelease=True,bForceImmediately=False,bNotifyUserSettings=False)"))))

(event Collision|EventActorBeginOverlap
  (params (OtherActor :type Actor%20Object%20Reference))
  (if (Utilities|Array|ContainsItem (Variables|/Script/Engine.Actor|GetTags OtherActor) "Enemy")
    (CallFunction|GetDamage)
    (elif (Utilities|Array|ContainsItem (Variables|/Script/Engine.Actor|GetTags OtherActor) "Shoot")
      (if (>= (- (Variables|Default|GetFireTemp) 0.8) 0.1)
        (Variables|Default|SetFireTemp (- (Variables|Default|GetFireTemp) 0.8))))))

(event EventTick
  (params (DeltaSeconds :type Float%20%28single-precision%29)))

(fn ConstructionScript)

(fn DoFire
  (Game|SpawnActorfromClass (Variables|Default|GetAmmo) (Transformation|GetWorldTransform (Variables|Default|GetShootPoint)) "Undefined" "MultiplyWithRoot" 0 0))