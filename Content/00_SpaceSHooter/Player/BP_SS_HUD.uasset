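; BP_SS_HUD is the space shooter's HUD, which creates and displays the game's user widget.
; On BeginPlay it adds BP_SS_UserWidget to the viewport and caches the player character and SS_GameMode.
; Every Tick it pushes the game mode's Progress and Level and the character's Lifes into the widget.
; Its PlayerKilled event forwards the death notice to the widget.
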(event Custom|PlayerKilled
  (Default|PlyerKilled (Variables|Default|GetGameWidget)))

(event EventBeginPlay
  (bind _returnvalue (Game|GetPlayerController 0))
  (Utilities|IsValid _returnvalue
    (:Is%20Valid
      (bind _returnvalue_2 (UserInterface|CreateWidget "/Game/00_SpaceSHooter/Player/BP_SS_UserWidget.BP_SS_UserWidget_C" _returnvalue))
      (bind _output_get (Variables|Default|SetGameWidget _returnvalue_2))
      (UserInterface|Viewport|AddtoViewport _output_get 0)
      (bind _asbp_sscharacter (Utilities|Casting|CastToBP_SSCharacter (Game|GetPlayerCharacter 0)))
      (Variables|Default|SetAs%20BP%20SSCharacter _asbp_sscharacter)
      (bind _asss_game_mode (Utilities|Casting|CastToSS_GameMode (Game|GetGameMode)))
      (Variables|Default|SetAs%20SS%20Game%20Mode _asss_game_mode))))

(event Collision|EventActorBeginOverlap
  (params (OtherActor :type Actor%20Object%20Reference)))

(event EventTick
  (params (DeltaSeconds :type Float%20%28single-precision%29))
  (bind _as_ss_game_mode (Variables|Default|GetAs%20SS%20Game%20Mode))
  (Default|UpdateWidget (Variables|Default|GetGameWidget) (Variables|/Game/00_SpaceSHooter/SS_GameMode.SS_GameMode_C|GetProgress _as_ss_game_mode) (Variables|/Game/00_SpaceSHooter/Player/BP_SSCharacter.BP_SSCharacter_C|GetLifes (Variables|Default|GetAs%20BP%20SSCharacter)) (Variables|/Game/00_SpaceSHooter/SS_GameMode.SS_GameMode_C|GetLevel _as_ss_game_mode)))

(fn ConstructionScript)