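; BP_RandomGen is the enemy spawner for the space shooter, driven by a BeginPlay timer that loops if SpawnerActive.
; Below level 4, it spawns a random enemy class, with variety capped by game mode level, at a random "SpawnPoint"-tagged component.
; From level 4, it spawns the boss at Point1 after a delay and destroys itself.
; Enemy deaths reduce SpawnTime, but the timer is never reset to use it.
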(event Custom|Spawn
  (if (< (Variables|/Game/00_SpaceSHooter/SS_GameMode.SS_GameMode_C|GetLevel (Variables|Default|Getm_GameMode)) 4)
    (bind _enemyspawned (CallFunction|SpawnEnemy))
    (EventDispatchers|BindEventtoOnEnemyDestroy _enemyspawned (delegate Custom|EnemyDestroyed))
    (else
      (Utilities|FlowControl|Delay 3.0)
      (Game|SpawnActorfromClass "/Game/00_SpaceSHooter/SS_BP_BOSS.SS_BP_BOSS_C" (Transformation|GetWorldTransform (Variables|Default|GetPoint1)) "Undefined" "MultiplyWithRoot" 0 0)
      (Actor|DestroyActor))))

(event Custom|EnemyDestroyed
  (Variables|Default|SetSpawnTime (- (Variables|Default|GetSpawnTime) 1.0)))

(event EventBeginPlay
  (Utilities|Time|SetTimerbyEvent (delegate Custom|Spawn) (Variables|Default|GetSpawnTime) (Variables|Default|GetSpawnerActive))
  (bind _asss_game_mode (Utilities|Casting|CastToSS_GameMode (Game|GetGameMode)))
  (Variables|Default|Setm_GameMode _asss_game_mode))

(event Collision|EventActorBeginOverlap
  (params (OtherActor :type Actor%20Object%20Reference)))

(event EventTick
  (params (DeltaSeconds :type Float%20%28single-precision%29)))

(fn ConstructionScript)

(fn SpawnEnemy
  (bind _returnvalue (Actor|GetComponentsbyTag "/Script/Engine.SceneComponent" "SpawnPoint"))
  (bind _class (CallFunction|GetClasstoSpawn (Math|Random|RandomInteger (Variables|/Game/00_SpaceSHooter/SS_GameMode.SS_GameMode_C|GetLevel (Variables|Default|Getm_GameMode)))))
  (bind _returnvalue_2 (Game|SpawnActorfromClass _class (Transformation|GetWorldTransform (Utilities|Array|Get(acopy) _returnvalue (Math|Random|RandomInteger (Utilities|Array|Length _returnvalue)))) "Undefined" "MultiplyWithRoot" 0 0))
  (return _returnvalue_2))

(fn GetClasstoSpawn
  (params (Type :type Integer))
  (return (Utilities|Select :Index (Math|Integer|Clamp(Integer) Type 0 (- (Variables|Default|GetMaxNumEnemies) 1)) :Option%200 "/Game/00_SpaceSHooter/SS_BP_Enemy.SS_BP_Enemy_C" :Option%201 "/Game/00_SpaceSHooter/SS_BP_Enemy2.SS_BP_Enemy2_C" :Option%202 "/Game/00_SpaceSHooter/SS_BP_EnemyTank.SS_BP_EnemyTank_C")))