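; BP_PowerUpSpawner is an actor that periodically spawns random power-ups in a space shooter.
; On BeginPlay it starts a looping timer at SpawnTime that calls ActualSpawnPowerUp.
; SpawnPowerUp picks one of three power-up classes with a random index bounded by PowerUpTypes.
; ActualSpawnPowerUp spawns that class at the world transform of a random scene component tagged SpawnPoint on the spawner.
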(event Custom|Spawn
  (CallFunction|ActualSpawnPowerUp))

(event EventBeginPlay
  (Utilities|Time|SetTimerbyEvent (delegate Custom|Spawn) (Variables|Default|GetSpawnTime) true))

(event Collision|EventActorBeginOverlap
  (params (OtherActor :type Actor%20Object%20Reference)))

(event EventTick
  (params (DeltaSeconds :type Float%20%28single-precision%29)))

(fn ConstructionScript)

(fn SpawnPowerUp
  (return (Utilities|Select :Index (Math|Random|RandomInteger (Variables|Default|GetPowerUpTypes)) :Option%200 "/Game/00_SpaceSHooter/PowerUpBase.PowerUpBase_C" :Option%201 "/Game/00_SpaceSHooter/PowerUp1.PowerUp1_C" :Option%202 "/Game/00_SpaceSHooter/PowerUp2.PowerUp2_C")))

(fn ActualSpawnPowerUp
  (bind _returnvalue (Actor|GetComponentsbyTag "/Script/Engine.SceneComponent" "SpawnPoint"))
  (bind _class (CallFunction|SpawnPowerUp))
  (bind _returnvalue_2 (Game|SpawnActorfromClass _class (Transformation|GetWorldTransform (Utilities|Array|Get(acopy) _returnvalue (Math|Random|RandomInteger (Utilities|Array|Length _returnvalue)))) "Undefined" "MultiplyWithRoot" 0 0))
  (return _returnvalue_2))